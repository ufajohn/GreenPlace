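; Game instance for the menu system that holds state shared with menus: startup video flag, save ID to load, menu settings and found sessions.
; It lazily spawns and caches a save manager actor and runs session searches that report success or failure through a dispatcher.
; It also opens the pause menu widget set in the menu settings, switching input mode and pausing only outside multiplayer, and closes it to restore gameplay.
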(event EventSetCanPlayVideo
  (params (canPlayVideo :type Boolean))
  ;[1 0.5609 0.1562] Set if the startup media can play.
  ; This variable tracks if the startup media is already played at startup or not.
  (Variables|Private|StartupMedia|SetbCanPlayVideo canPlayVideo))

(event EventFindSessions
  (params (MaxResults :type Integer) (bUseLan :type Boolean))
  ;[0 0 0] Networking               [Replace this stuff with Advanced Session plugin, for more functionality]
  ;;[0.04688 0.04688 0.04688] Find sessions
  (Utilities|Array|Clear (Variables|Private|Networking|GetSessions))
  (bind _results (|FindSessions (Game|GetPlayerController 0) MaxResults bUseLan)
    (:OnSuccess
      (Variables|Private|Networking|SetSessions _results)
      (Default|CallOnSessionsFound false))
    (:OnFailure
      (Default|CallOnSessionsFound true))))

(event EventSetMenuSettings
  (params (MenuSettings :type F%20Menu%20Settings%20Structure))
  (Variables|Settings|SetMenuSettings MenuSettings))

(event EventClosePauseMenu
  (bind _returnvalue (Game|GetPlayerController 0))
  ;[0 1 0.4244] Close pause menu and unpause game
  (Game|SetGamePaused false)
  (bind _pausemenureference (Variables|Private|Menu|GetPauseMenuReference)
    (:then
      (Widget|RemovefromParent _pausemenureference))
    (:else
      _))
  (Variables|/Script/Engine.PlayerController|SetbShowMouseCursor _returnvalue false)
  (Input|SetInputModeGameOnly _returnvalue)
  (Variables|Private|Menu|SetPauseMenuReference 0)
  (Variables|Private|Menu|SetbPauseMenuOpened false))

(event EventSetSaveIdtoLoad
  (params (SaveID :type String))
  ;[1 0.5609 0.1562] Save ID to load when the game loads
  (Variables|Private|SaveSystem|SetSaveID SaveID))

(fn GetCanPlayVideo
  (return (Variables|Private|StartupMedia|GetbCanPlayVideo)))

(fn GetIsPauseMenuOpened
  (return (Variables|Private|Menu|GetbPauseMenuOpened)))

(fn GetMenuSettings
  (return (Variables|Settings|GetMenuSettings)))

(fn GetSaveIDtoLoad
  (return (Variables|Private|SaveSystem|GetSaveID)))

(fn GetSaveManager
  (bind _savemanager (Variables|Private|SaveSystem|GetSaveManager)
    (:then
      (return _savemanager))
    (:else
      (bind _returnvalue (Game|SpawnActorfromClass "/Game/MenuSystem/Blueprints/SaveSystem/BP_save_manager.BP_save_manager_C" (Math|Transform|MakeTransform "0, 0, 0" "0, 0, 0" "1,1,1") "AlwaysSpawn" 0 0))
      (bind _output_get (Variables|Private|SaveSystem|SetSaveManager _returnvalue))
      (return _output_get))))

(fn GetSessions
  (return (Variables|Private|Networking|GetSessions)))

(fn OpenPauseMenu
  (bind _returnvalue (Game|GetPlayerController 0))
  (if (not (Utilities|IsValid (Variables|Private|Menu|GetPauseMenuReference)))
    _
    (else
      (Widget|RemovefromParent (Variables|Private|Menu|GetPauseMenuReference))))
  (bind _menusettings (Class|BPIGIAMS|GetMenuSettings(Message) (Game|GetGameInstance)))
  (bind _returnvalue_2 (UserInterface|CreateWidget (.PauseMenuToOpen (Utilities|Struct|BreakFMenuSettings _menusettings)) (Game|GetPlayerController 0)))
  (bind _output_get (Variables|Private|Menu|SetPauseMenuReference _returnvalue_2)) ; Create a referance so we can remove it
  (UserInterface|Viewport|AddtoViewport _output_get 0)
  (Widget|SetKeyboardFocus _returnvalue_2)
  (Input|SetInputModeUIOnly _returnvalue _returnvalue_2 "DoNotLock")
  (Variables|/Script/Engine.PlayerController|SetbShowMouseCursor _returnvalue true)
  (EventDispatchers|BindEventtoOnResumeGame _returnvalue_2 (EventDispatchers|CreateEvent :!event ClosePauseMenu))
  (Game|SetGamePaused (not (.bIsMultiplayer (Utilities|Struct|BreakFMenuSettings _menusettings))))
  (Variables|Private|Menu|SetbPauseMenuOpened true)
  (return (Variables|Private|Menu|GetPauseMenuReference)))