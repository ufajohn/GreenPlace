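; Blueprint function library of save-system wrappers for the menu system, mostly left as empty stubs.
; SaveGameWrapper writes the player character's transform to a BP_General_SaveGame in a fixed slot and prints a confirmation.
; LoadFromSaveIDWrapper ignores its SaveID and restores that transform from the same slot.
; The other wrappers return false or nothing; a disconnected warning refers to the uninstalled AGS Basic Save Game plugin.
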(fn GetSaveExistsWrapper
  (return false))

(fn SetSaveIDtoLoadWrapper
  (params (SaveID :type String)))

(fn IsLatestSaveIDWrapper
  (params (SaveID :type String))
  (return false))

(fn LoadfromLastCheckpointWrapper)

(fn SaveGameWrapper
  (bind _returnvalue (SaveGame|CreateSaveGameObject "/Game/MenuSystem/Blueprints/SaveObjects/BP_General_SaveGame.BP_General_SaveGame_C"))
  (Variables|/Game/MenuSystem/Blueprints/SaveObjects/BP_General_SaveGame.BP_General_SaveGame_C|SetCharTransform _returnvalue (Transformation|GetActorTransform (Game|GetPlayerCharacter 0)))
  (SaveGame|SaveGametoSlot _returnvalue "1")
  (Development|PrintString 0 "Игра сохранена" true true "(R=0.000000,G=0.660000,B=1.000000,A=1.000000)" 6e+01))

(fn LoadfromSaveIDWrapper
  (params (SaveID :type String))
  (bind _returnvalue (SaveGame|LoadGamefromSlot "1"))
  (bind _asbp_general_save_game (Utilities|Casting|CastToBP_General_SaveGame _returnvalue))
  (Transformation|SetActorTransform (Game|GetPlayerCharacter 0) (Variables|/Game/MenuSystem/Blueprints/SaveObjects/BP_General_SaveGame.BP_General_SaveGame_C|GetCharTransform _asbp_general_save_game)))

(fn RemoveAllSavesWrapper)

(fn GetSaveListWrapper
  (return 0))

(fn GetSavableActorListWrapper
  (return 0))

(fn GetSaveManager
  (return false 0))